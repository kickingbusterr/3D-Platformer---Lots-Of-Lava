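; Shield pickup that flies onto the player who overlaps its sphere and enables their shield ability.
; On overlap it removes its idle movement and effect components, flags the player controller as having had a shield, then uses a timeline to lerp to the mesh's shield socket.
; It then attaches, plays an energy burst, spawns a pickup notification and binds its own destruction to the player's death dispatch.
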(event `Picked Up`
  (params (Player :type "/Game/Blueprints/PlayerCharacter Object Reference"))
  (bind _returnvalue_location (`KismetMathLibrary.BreakTransform` (`self.GetTransform`)))
  (bind _mesh (`Character.Mesh` Player))
  (bind (_returnvalue_location_2 _returnvalue_rotation) (`KismetMathLibrary.BreakTransform` (`SceneComponent.GetSocketTransform` _mesh "ShieldAttachSocket" "RTS_World")))
  (`ActorComponent.K2_DestroyComponent` (`self.InterpToMovement`))
  (`ActorComponent.K2_DestroyComponent` (`self.RotatingMovement`))
  (`ActorComponent.K2_DestroyComponent` (`self.Sphere`))
  (`ActorComponent.K2_DestroyComponent` (`self.Floating_EnergySystem`))
  (bind _asbp_sem_1player_controller (cast `/Game/Blueprints/MiscBlueprints/BP_Sem1PlayerController` (`Pawn.GetController` Player)))
  (set `/Game/Blueprints/MiscBlueprints/BP_Sem1PlayerController.PlayerHadShield` true _asbp_sem_1player_controller)
  (set `self.StartRotation` (`self.K2_GetActorRotation`))
  (set `self.StartLocation` (`self.K2_GetActorLocation`))
  (bind (_direction _alpha) (`Timeline|PickedUpTL` :!via `PlayFromStart`)
    (:`Update`
      (`self.K2_SetActorLocation` (`KismetMathLibrary.VLerp` (`self.StartLocation`) _returnvalue_location_2 _alpha))
      (`self.K2_SetActorRotation` (`KismetMathLibrary.RLerp` (`self.StartRotation`) _returnvalue_rotation _alpha)))
    (:`Finished`
      (`self.K2_AttachToComponent` _mesh "ShieldAttachSocket" "SnapToTarget" "SnapToTarget" "KeepWorld")
      (set `/Game/Blueprints/PlayerCharacter.CanShield` true Player)
      (`NiagaraFunctionLibrary.SpawnSystemAtLocation` "/Game/Emitters/NS_EnergyBurst.NS_EnergyBurst" (`self.K2_GetActorLocation`) (`KismetMathLibrary.NegateRotator` (`self.K2_GetActorRotation`)))
      (`|SpawnActorFromClass` "/Game/UI/WBP_PickUpNotification.WBP_PickUpNotification_C" (`KismetMathLibrary.MakeTransform` _returnvalue_location) "AlwaysSpawn" "OverrideRootScale" null "Shield Collected!" null)
      (add `/Game/Blueprints/PlayerCharacter.DeathDispatch` Player (delegate `Destroy self`)))))

(event `Destroy self`
  (`self.K2_DestroyActor`))

(event `self.Sphere.OnComponentBeginOverlap`
  (params (OverlappedComponent :type "PrimitiveComponent Object Reference") (OtherActor :type "Actor Object Reference") (OtherComp :type "PrimitiveComponent Object Reference") (OtherBodyIndex :type Integer) (bFromSweep :type Boolean) (SweepResult :type "HitResult Structure (by ref)"))
  (bind _asplayer_character (cast `/Game/Blueprints/PlayerCharacter` OtherActor))
  (`self.Picked Up` _asplayer_character))

(fn `UserConstructionScript`)